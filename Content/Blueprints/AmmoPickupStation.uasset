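; AmmoPickupStation is a respawning pickup that grants ammo to the player character.
; When an SPfpsMovementCharacter without ammo overlaps the Canister, it sets that character's HasAmmo flag.
; The Canister then hides and disables collision, and after a RespawnTime delay reappears with query-only collision.
; Characters that already have ammo leave the pickup untouched.
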(event `self.ReceiveTick`
  (params (DeltaSeconds :type "Float (single-precision)")))

(event `self.Canister.OnComponentBeginOverlap`
  (params (OtherActor :type "Actor Object Reference") (OtherComp :type "PrimitiveComponent Object Reference") (OtherBodyIndex :type Integer) (bFromSweep :type Boolean) (SweepResult :type "HitResult Structure (by ref)"))
  (bind _asspfps_movement_character (cast `/Game/Blueprints/SPfpsMovementCharacter` OtherActor))
  (if (not (`/Game/Blueprints/SPfpsMovementCharacter.HasAmmo` _asspfps_movement_character))
    (set `/Game/Blueprints/SPfpsMovementCharacter.HasAmmo` true _asspfps_movement_character)
    (`SceneComponent.SetVisibility` (`self.Canister`) false true)
    (`PrimitiveComponent.SetCollisionEnabled` (`self.Canister`) "NoCollision")
    (`KismetSystemLibrary.Delay` (`self.RespawnTime`))
    (`SceneComponent.SetVisibility` (`self.Canister`) true true)
    (`PrimitiveComponent.SetCollisionEnabled` (`self.Canister`) "QueryOnly")))

(fn `UserConstructionScript`)