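; Checkpoint actor that records the player's respawn location and rotation on a linked RespawnTrigger when an SPfpsMovementCharacter overlaps it.
; Each Tick it compares the trigger's current checkpoint to its own location, turning its point light green when active and red otherwise.
; The construction script applies the configurable Size to the box and aims the arrow along CheckpointRotation to preview the respawn facing.
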(event `self.ReceiveBeginPlay`)

(event `self.ReceiveTick`
  (params (DeltaSeconds :type "Float (single-precision)"))
  (bind _pointlight (`self.PointLight`))
  (if (== (`/Game/Blueprints/RespawnTrigger.CurrentCheckpoint` (`self.RespawnTrigger`)) (`self.K2_GetActorLocation`))
    (`LightComponent.SetLightColor` _pointlight (struct :`R` 0.001891 :`G` 1.0 :`A` 1.0) true)
    (else
      (`LightComponent.SetLightColor` _pointlight (struct :`R` 1.0 :`B` 0.05564 :`A` 1.0) true))))

(event `self.ReceiveActorBeginOverlap`
  (params (OtherActor :type "Actor Object Reference"))
  (bind _respawntrigger (`self.RespawnTrigger`))
  (cast `/Game/Blueprints/SPfpsMovementCharacter` OtherActor)
  (set `/Game/Blueprints/RespawnTrigger.CurrentCheckpoint` (`self.K2_GetActorLocation`) _respawntrigger)
  (set `/Game/Blueprints/RespawnTrigger.CurrentCheckPointRotation` (`self.CheckpointRotation`) _respawntrigger))

(fn `UserConstructionScript`
  (`SceneComponent.K2_SetWorldRotation` (`self.Arrow`) (`self.CheckpointRotation`) false false)
  (`BoxComponent.SetBoxExtent` (`self.Box`) (`self.Size`) true))